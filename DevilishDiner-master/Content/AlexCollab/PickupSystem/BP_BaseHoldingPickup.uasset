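; Base pickup actor that a player character carries on the mesh's HeldObject socket, tracked through the character's plate-holding state.
; Overlapping InteractVolume with no plate and a matching held-tool state binds the controller's HUD interact and drop events; leaving unbinds only interact.
; Pickup attaches the actor and disables the volume's collision.
; Drop detaches it at the character's location, restores collision and clears the character reference.
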(event `self.InteractVolume.OnComponentBeginOverlap`
  (params (OverlappedComponent :type "PrimitiveComponent Object Reference") (OtherActor :type "Actor Object Reference") (OtherComp :type "PrimitiveComponent Object Reference") (OtherBodyIndex :type Integer) (bFromSweep :type Boolean) (SweepResult :type "HitResult Structure (by ref)"))
  (`/Game/JayCollab/Interfaces/BP_MacroLibrary.IsPlayer?` OtherActor
    (:`IsPlayer`
      (bind _asbp_base_character (cast `/Game/JayCollab/BP_BaseCharacter` OtherActor))
      (if (`|EnumEquality` (`/Game/JayCollab/BP_BaseCharacter.CurrentHeldTool` _asbp_base_character) "NewEnumerator0")
        (`/Game/JayCollab/BP_BaseCharacter.Held Plate` _asbp_base_character
          (:`then`)
          (:`else`
            (bind _output_get (set `self.Character` _asbp_base_character))
            (if (not (`/Game/JayCollab/BP_BaseCharacter.HasPlate` _output_get))
              (bind _asbp_base_controller (cast `/Game/JayCollab/BP_BaseController` (`Pawn.GetController` _asbp_base_character)))
              (set `self.Controller` _asbp_base_controller)
              (add `/Game/JayCollab/BP_BaseController.ED_HUDInteract` _asbp_base_controller (`|CreateDelegate` :!event `F_PickUpObject`))
              (add `/Game/JayCollab/BP_BaseController.ED_HUDDropItem` _asbp_base_controller (`|CreateDelegate` :!event `F_DropObject`)))))))))

(event `self.InteractVolume.OnComponentEndOverlap`
  (params (OverlappedComponent :type "PrimitiveComponent Object Reference") (OtherActor :type "Actor Object Reference") (OtherComp :type "PrimitiveComponent Object Reference") (OtherBodyIndex :type Integer))
  (`/Game/JayCollab/Interfaces/BP_MacroLibrary.IsPlayer?` OtherActor
    (:`IsPlayer`
      (bind _controller (`self.Controller`)
        (:`then`
          (remove `/Game/JayCollab/BP_BaseController.ED_HUDInteract` _controller (`|CreateDelegate` :!event `F_PickUpObject`)))
        (:`else`)))))

(fn `F_DropObject`
  (bind _character (`self.Character`)
    (:`then`
      (if (`/Game/JayCollab/BP_BaseCharacter.HasPlate` _character)
        (set `/Game/JayCollab/BP_BaseCharacter.HasPlate` false _character)
        (`/Game/JayCollab/BP_BaseCharacter.Set Current Held Plate` (`self.Character`) null)
        (`self.K2_DetachFromActor` "KeepRelative")
        (`self.K2_SetActorLocation` (`self.K2_GetActorLocation` _character))
        (`PrimitiveComponent.SetCollisionEnabled` (`self.InteractVolume`) "QueryAndPhysics")
        (set `self.Character` null)))
    (:`else`)))

(fn `F_PickUpObject`
  (bind _character (`self.Character`)
    (:`then`
      (`/Game/JayCollab/BP_BaseCharacter.Held Plate` _character
        (:`then`)
        (:`else`
          (if (`/Game/JayCollab/BP_BaseCharacter.HasPlate` _character)
            _
            (elif (`|EnumEquality` (`/Game/JayCollab/BP_BaseCharacter.CurrentHeldTool` _character) "NewEnumerator0")
              (`self.K2_AttachToComponent` (`Character.Mesh` _character) "HeldObject" "SnapToTarget" "SnapToTarget" "KeepWorld")
              (set `/Game/JayCollab/BP_BaseCharacter.HasPlate` true (`self.Character`))
              (`PrimitiveComponent.SetCollisionEnabled` (`self.InteractVolume`) "NoCollision")
              (else
                (`self.F_DropObject`)))))))
    (:`else`)))

(fn `UserConstructionScript`
  (`parent.UserConstructionScript`))