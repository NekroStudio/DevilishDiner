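; BP_Counter is a pickup-system counter that holds a single docked plate and receives its PlateManager through Init.
; SpawnPlate creates a BP_Plate at the Arrow component's location when free, passing it the counter, delivery point and HUD manager, then marks itself docked.
; ClearCounter resets that flag to allow another spawn, and IPlateDocked exposes the occupied state.
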(event `Init`
  (params (`Plate Manager` :type "/Game/AlexCollab/PickupSystem/BP_PlateManager Object Reference"))
  (set `self.Plate Manager` `Plate Manager`))

(event `ClearCounter`
  (set `self.PlateDocked` false))

(fn `I_PlateDocked`
  (returns (PlateDocked :type Boolean))
  (return (`self.PlateDocked`)))

(fn `Spawn Plate`
  (params (`Delivery Point` :type "/Game/AlexCollab/PickupSystem/BP_DeliveryPoint Object Reference") (`HUD Manager` :type "/Game/AlexCollab/HUD_Manager Object Reference"))
  (bind _returnvalue_location (`KismetMathLibrary.BreakTransform` (`SceneComponent.K2_GetComponentToWorld` (`self.Arrow`))))
  (if (not (`self.PlateDocked`))
    (bind _returnvalue (`|SpawnActorFromClass` "/Game/AlexCollab/PickupSystem/BP_Plate.BP_Plate_C" (`KismetMathLibrary.MakeTransform` _returnvalue_location) "Undefined" "OverrideRootScale" null null))
    (`/Game/AlexCollab/PickupSystem/BP_Plate.Init` _returnvalue self `Delivery Point` `HUD Manager`))
  (set `self.PlateDocked` true))

(fn `UserConstructionScript`)