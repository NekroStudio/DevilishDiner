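; Manager for plate deliveries that pairs a counter with a random delivery point.
; Shortly after BeginPlay it finds the HUD manager, then registers and initializes all counters and delivery points with IDs.
; CreateDelivery re-rolls until a point is untaken with a valid, unfilled linked chair, then has the counter spawn a plate for it.
; Rejected points are logged in a never-cleared list, printing an abort message once it covers all points.
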(event `self.ReceiveBeginPlay`
  (`KismetSystemLibrary.Delay` 0.5)
  (`self.Init`))

(event `Init`
  (bind _foundwidgets (`WidgetBlueprintLibrary.GetAllWidgetsOfClass` "/Game/AlexCollab/HUD_Manager.HUD_Manager_C"))
  (set `self.HUD Manager` (`|GetArrayItem` _foundwidgets))
  (`self.Init Delivery Points`)
  (`self.Init Counters`))

(event `ClearValues`
  (`KismetSystemLibrary.Delay` 1.0)
  (set `self.Delivery Point To Be Assigned` null)
  (set `self.Counter To Be Assigned` null)
  (set `self.Loop Delivery Point` null))

(fn `Check number of free Delivery Points`
  (params (`Delivery Point` :type "/Game/AlexCollab/PickupSystem/BP_DeliveryPoint Object Reference (by ref)"))
  (bind _taken_delivery_points (`self.Taken Delivery Points`))
  (`KismetArrayLibrary.Array_AddUnique` _taken_delivery_points `Delivery Point`)
  (if (== (`KismetArrayLibrary.Array_Length` _taken_delivery_points) (`KismetArrayLibrary.Array_Length` (`self.Delivery Points`)))
    (`KismetSystemLibrary.PrintString` "ALL DELIVERY POINTS TAKEN. ABORTING.")
    (else
      (return))))

(fn `Create Delivery`
  (params (Counter :type "/Game/AlexCollab/PickupSystem/BP_Counter Object Reference"))
  (returns (`Delivery Point To Be Assigned` :type "/Game/AlexCollab/PickupSystem/BP_DeliveryPoint Object Reference"))
  (locals (Successful :type Boolean))
  (bind _delivery_point_to_be_assigned (`self.Delivery Point To Be Assigned`))
  (set `self.Counter To Be Assigned` Counter)
  (bind (_deliverypoint _taken) (`self.Get Random Delivery Point` :!label _label))
  (if (not _taken)
    (bind _linkedchair (`/Game/AlexCollab/PickupSystem/BP_DeliveryPoint.LinkedChair` _deliverypoint)
      (:`then`
        (if (`/Game/JayCollab/Blueprints/ChairLocations/BP_ChairLocation.ChairIsFull` _linkedchair)
          _
          (else
            (set `self.Delivery Point To Be Assigned` _deliverypoint)
            (`/Game/AlexCollab/PickupSystem/BP_Counter.Spawn Plate` (`self.Counter To Be Assigned`) _delivery_point_to_be_assigned (`self.HUD Manager`))
            (`self.ClearValues`)
            (return _delivery_point_to_be_assigned))))
      (:`else`
        _)))
  (`self.Check number of free Delivery Points` _deliverypoint)
  (goto _label))

(fn `Get Random Delivery Point`
  (returns (DeliveryPoint :type "/Game/AlexCollab/PickupSystem/BP_DeliveryPoint Object Reference") (Taken :type Boolean))
  (bind _delivery_points (`self.Delivery Points`))
  (bind _output (`|GetArrayItem` _delivery_points (`KismetMathLibrary.RandomInteger` (`KismetArrayLibrary.Array_Length` _delivery_points))))
  (return _output (`/Game/AlexCollab/PickupSystem/BP_DeliveryPoint.Delivery Point Taken` _output)))

(fn `Init Counters`
  (bind _outactors (`GameplayStatics.GetAllActorsOfClass` "/Game/AlexCollab/PickupSystem/BP_Counter.BP_Counter_C"))
  (for _array_element _outactors
    (bind _returnvalue (`KismetArrayLibrary.Array_AddUnique` (`self.Counters`) _array_element))
    (set `/Game/AlexCollab/PickupSystem/BP_Counter.ID` _returnvalue _array_element)
    (`/Game/AlexCollab/PickupSystem/BP_Counter.Init` _array_element self)))

(fn `Init Delivery Points`
  (bind _outactors (`GameplayStatics.GetAllActorsOfClass` "/Game/AlexCollab/PickupSystem/BP_DeliveryPoint.BP_DeliveryPoint_C"))
  (for _array_element _outactors
    (bind _returnvalue (`KismetArrayLibrary.Array_AddUnique` (`self.Delivery Points`) _array_element))
    (set `/Game/AlexCollab/PickupSystem/BP_DeliveryPoint.ID` _returnvalue _array_element)
    (`/Game/AlexCollab/PickupSystem/BP_DeliveryPoint.Init` _array_element self)))

(fn `UserConstructionScript`)