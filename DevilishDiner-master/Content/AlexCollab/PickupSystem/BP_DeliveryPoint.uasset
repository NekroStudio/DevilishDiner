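; Delivery point actor where players hand plates to the customer on a linked chair.
; Player overlap binds the controller's interact event, and a dynamic material colour shows whether the point is current, eating or idle.
; Delivery checks the held plate targets this point, attaches it, awards points and notifies the customer.
; A timer then destroys the plate, resets the point, triggers customer exit with happy or sad Niagara effects, and decreases the chair count.
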(event `CurrentlyEating`
  (`MaterialInstanceDynamic.SetVectorParameterValue` (`self.Material`) "Colour" (struct :`R` 0.119631 :`G` 0.123744 :`B` 0.125 :`A` 1.0))
  (set `self.Delivery Point Taken` true))

(event `Is Not Current Delivery Point`
  (bind _linkedchair (`self.LinkedChair`))
  (`MaterialInstanceDynamic.SetVectorParameterValue` (`self.Material`) "Colour" (struct :`G` 0.003922 :`B` 0.05098 :`A` 1.0))
  (set `self.Delivery Point Taken` false)
  (message `/Game/JayCollab/Blueprints/ChairLocations/BPI_CustomerTableInfo.I_CustomerExit` _linkedchair)
  (bind _customerhappy (message `/Game/JayCollab/AI/BPI_CustomerInterface.I_CheckCustomerIsHappy` (`/Game/JayCollab/Blueprints/ChairLocations/BP_ChairLocation.CurrentCustomer` _linkedchair)))
  (if _customerhappy
    (bind _returnvalue (`NiagaraFunctionLibrary.SpawnSystemAtLocation` "/Game/JayCollab/FX/NS_HappyCustomerLeavingFX.NS_HappyCustomerLeavingFX" (`self.K2_GetActorLocation`) (struct) (0.5 0.5 0.5)))
    (`KismetSystemLibrary.Delay` 0.2)
    (`ActorComponent.Deactivate` _returnvalue)
    (else
      (bind _returnvalue_2 (`NiagaraFunctionLibrary.SpawnSystemAtLocation` "/Game/JayCollab/FX/NS_SadCustomerLeavingFX.NS_SadCustomerLeavingFX" (`self.K2_GetActorLocation`) (struct) (0.5 0.5 0.5)))
      (`KismetSystemLibrary.Delay` 0.2)
      (`ActorComponent.Deactivate` _returnvalue_2))))

(event `Is Current Delivery Point`
  (params (Value :type "LinearColor Structure"))
  (`MaterialInstanceDynamic.SetVectorParameterValue` (`self.Material`) "Colour" Value)
  (set `self.Delivery Point Taken` true))

(event `Init`
  (params (`Plate Manager` :type "/Game/AlexCollab/PickupSystem/BP_PlateManager Object Reference"))
  (set `self.PlateManager` `Plate Manager`)
  (bind _returnvalue (`PrimitiveComponent.CreateDynamicMaterialInstance` (`self.Cube`) 0 null "None"))
  (set `self.Material` _returnvalue)
  (`TextRenderComponent.K2_SetText` (`self.TextRender`) (`KismetTextLibrary.Conv_IntToText` (`self.ID`))))

(event `self.InteractVolume.OnComponentBeginOverlap`
  (params (OverlappedComponent :type "PrimitiveComponent Object Reference") (OtherActor :type "Actor Object Reference") (OtherComp :type "PrimitiveComponent Object Reference") (OtherBodyIndex :type Integer) (bFromSweep :type Boolean) (SweepResult :type "HitResult Structure (by ref)"))
  (`/Game/JayCollab/Interfaces/BP_MacroLibrary.IsPlayer?` OtherActor
    (:`IsPlayer`
      (bind _asbp_base_character (cast `/Game/JayCollab/BP_BaseCharacter` OtherActor))
      (bind _asbp_base_controller (cast `/Game/JayCollab/BP_BaseController` (`Pawn.GetController` _asbp_base_character)))
      (set `self.Base Controller` _asbp_base_controller)
      (set `self.Character` _asbp_base_character)
      (add `/Game/JayCollab/BP_BaseController.ED_HUDInteract` _asbp_base_controller (`|CreateDelegate` :!event `F_DeliverPlate`)))))

(event `self.InteractVolume.OnComponentEndOverlap`
  (params (OverlappedComponent :type "PrimitiveComponent Object Reference") (OtherActor :type "Actor Object Reference") (OtherComp :type "PrimitiveComponent Object Reference") (OtherBodyIndex :type Integer))
  (`/Game/JayCollab/Interfaces/BP_MacroLibrary.IsPlayer?` OtherActor
    (:`IsPlayer`
      (remove `/Game/JayCollab/BP_BaseController.ED_HUDInteract` (`self.Base Controller`) (`|CreateDelegate` :!event `F_DeliverPlate`)))))

(fn `F_DeliverPlate`
  (bind _points_value (`self.Points Value`))
  (bind _attachedplate (`self.AttachedPlate`))
  (bind _character (`self.Character`))
  (bind _currentcustomer (`/Game/JayCollab/Blueprints/ChairLocations/BP_ChairLocation.CurrentCustomer` (`self.LinkedChair`)))
  ;[1 1 1] Check this is the right Delivery Point
  (bind _character_2 (`self.Character`)
    (:`then`
      (bind _held_plate (`/Game/JayCollab/BP_BaseCharacter.Held Plate` _character_2)
        (:`then`
          (if (== (`/Game/AlexCollab/PickupSystem/BP_Plate.Delivery Point` _held_plate) self)
            ;[1 1 1] Attach Plate to Delivery Point
            (bind _output_get (set `self.AttachedPlate` _held_plate))
            (`self.K2_AttachToComponent` _output_get (`self.Arrow`) "None" "SnapToTarget" "KeepRelative" "KeepRelative" true)
            (`self.K2_SetActorRotation` :`self` _output_get)
            (set `self.Delivery Point Taken` true)
            (`self.CurrentlyEating`)
            (`/Game/JayCollab/BP_BaseCharacter.HUD_Hide Thought Bubble` (`self.Character`))
            ;[1 1 1] Null Player Plate Values
            (set `/Game/AlexCollab/PickupSystem/BP_BaseHoldingPickup.Character` null (`self.AttachedPlate`))
            (set `/Game/JayCollab/BP_BaseCharacter.Held Plate` null _character)
            (set `/Game/JayCollab/BP_BaseCharacter.HasPlate` false _character)
            ;[1 1 1] Adjust points based on food quality
            (set `self.Points Value` (`self.M_CalcPoints`))
            ;[1 1 1] Stop plate taking damage
            (set `/Game/AlexCollab/PickupSystem/BP_Plate.CanTakeDamage` false (`self.AttachedPlate`))
            ;[1 1 1] Notify Other Objects of Delivery Completion
            (message `/Game/JayCollab/Interfaces/BPI_TableAndPointsSystem.I_ModifyPoints` (`GameplayStatics.GetGameMode`) true _points_value)
            (`self.DeliveryCompleted` _points_value)
            (`/Game/AlexCollab/HUD_PlateFrame.DeliveryFinished` (`/Game/AlexCollab/PickupSystem/BP_Plate.Frame` (`self.AttachedPlate`)))
            ;;[1 1 1] Stop plate quality decreasing
            (`/Game/AlexCollab/PickupSystem/BP_Plate.I_PausePlateQuality` _attachedplate)
            (set `/Game/AlexCollab/PickupSystem/BP_Plate.FoodQuality` null _attachedplate)
            ;[1 1 1] Send customer happy - Start eating
            (message `/Game/JayCollab/AI/BPI_CustomerInterface.I_CustomerIsHappy` _currentcustomer)
            (bind _customer (message `/Game/MathieuLecerfCollab/AnimationFolder/AnimationFolder/AnimationBP/BPI_CustomerAnimations.I_GetCustomer` _currentcustomer))
            (set `/Game/JayCollab/AI/BP_Customer.State` "NewEnumerator2" _customer)
            ;[1 1 1] Null Character Ref
            (set `self.Character` null)
            ;[1 1 1] Despawn Plate Timer
            (`KismetSystemLibrary.K2_SetTimer` self "F_DespawnPlate" 4.0)))
        (:`else`)))
    (:`else`)))

(fn `F_DespawnPlate`
  (bind _attachedplate (`self.AttachedPlate`)
    (:`then`
      (`self.K2_DestroyActor` _attachedplate))
    (:`else`
      _))
  (`self.Is Not Current Delivery Point`)
  (message `/Game/JayCollab/Blueprints/ChairLocations/BPI_CustomerTableInfo.I_CustomerExit` (`self.LinkedChair`))
  (message `/Game/JayCollab/Interfaces/BPI_TableAndPointsSystem.I_DecreaseChairAmount` (`GameplayStatics.GetGameMode`)))

(fn `UserConstructionScript`)