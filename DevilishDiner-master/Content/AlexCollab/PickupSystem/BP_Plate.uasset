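; BP_Plate is a carryable food plate tied to a counter and delivery point, which fails when it goes cold or runs out of health.
; A looping, pausable timer drains heat, with Niagara steam or fire effects, and Init adds a HUD frame that follows pickup and drop state, showing the carrier's scene capture.
; Failure clears the counter and delivery point, spawns a hazard if carried, deducts points and destroys the plate.
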(event `/Game/JayCollab/BPI_PlateCommunication.I_PausePlateQuality`
  (`KismetSystemLibrary.K2_PauseTimerHandle` (`self.PlateQualityHandle`)))

(event `Init`
  (params (`Parent Counter` :type "/Game/AlexCollab/PickupSystem/BP_Counter Object Reference") (`Delivery Point` :type "/Game/AlexCollab/PickupSystem/BP_DeliveryPoint Object Reference") (`HUD Manager` :type "/Game/AlexCollab/HUD_Manager Object Reference"))
  ;[1 1 1] Init
  (set `self.Parent Counter` `Parent Counter`)
  (set `self.Delivery Point` `Delivery Point`)
  (bind _returnvalue (`|CreateWidget` "/Game/AlexCollab/HUD_PlateFrame.HUD_PlateFrame_C" (`GameplayStatics.GetPlayerController` 0)))
  (`UserWidget.AddToViewport` _returnvalue 0)
  (`HorizontalBox.AddChildToHorizontalBox` (`/Game/AlexCollab/HUD_Manager.HorizontalBox_0` `HUD Manager`) _returnvalue)
  (`/Game/AlexCollab/HUD_PlateFrame.Init` _returnvalue (`/Game/AlexCollab/PickupSystem/BP_DeliveryPoint.ID` (`self.Delivery Point`)) self)
  (bind _output_get (set `self.Frame` _returnvalue))
  (`WidgetSwitcher.SetActiveWidgetIndex` (`/Game/AlexCollab/HUD_PlateFrame.IconState` _output_get) 0))

(event `/Game/JayCollab/BPI_PlateCommunication.I_ResumePlateQuality`
  (`KismetSystemLibrary.K2_UnPauseTimerHandle` (`self.PlateQualityHandle`)))

(event `TriggerPlateCooling`
  (bind _returnvalue (`KismetSystemLibrary.K2_SetTimerDelegate` (delegate `EventCurrentPlateHeat`) 0.01 true))
  (set `self.PlateQualityHandle` _returnvalue))

(event `TriggerFireFX`
  (bind _niagarafx (`self.NiagaraFX`))
  ;[1 1 1] Fire FX
  (`NiagaraComponent.SetAsset` _niagarafx "/Game/JayCollab/FX/NS_FireFX_System.NS_FireFX_System")
  (`ActorComponent.Activate` _niagarafx true))

(event `self.ReceiveBeginPlay`
  (bind _returnvalue (`KismetMathLibrary.RandomFloat`))
  ;[1 1 1] Bgein play, store current plate health
  (`parent.ReceiveBeginPlay`)
  (set `self.Linear Color` (make `LinearColor` _returnvalue (`KismetMathLibrary.RandomFloat`) _returnvalue 1.0))
  (`self.F_SetPlateVariables`)
  (`NiagaraComponent.SetAsset` (`self.NiagaraFX`) "/Game/JayCollab/FX/NS_SteamFX_System.NS_SteamFX_System")
  (`self.TriggerPlateCooling`))

(event `EventCurrentPlateHeat`
  (set `self.CurrentPlateQuality` (- (`self.CurrentPlateQuality`) (`self.PlateQualityDeduction`)))
  (if (<= (`self.CurrentPlateQuality`) 0.0)
    (`KismetSystemLibrary.PrintString` "cold")
    (`self.PlateIsCold`)
    (`KismetSystemLibrary.K2_ClearAndInvalidateTimerHandle` (`self.PlateQualityHandle`))
    (else
      (`KismetSystemLibrary.PrintString` (`KismetStringLibrary.Concat_StrStr` "Current Heat: " (`KismetStringLibrary.Conv_DoubleToString` (`self.CurrentPlateQuality`))) true true (`self.Linear Color`))
      (if (`self.M_PlateGettingTooCold?`)
        (`/Engine/EditorBlueprintResources/StandardMacros.DoOnce` false
          (:`Completed`
            (`ActorComponent.Deactivate` (`self.NiagaraFX`))))))))

(event `RemoveFireEffect`
  (bind _niagarafx (`self.NiagaraFX`))
  ;[1 1 1] Fire FX
  (`ActorComponent.Deactivate` _niagarafx)
  (`KismetSystemLibrary.Delay` 2.0)
  (if (not (`self.M_PlateGettingTooCold?`))
    (`NiagaraComponent.SetAsset` _niagarafx "/Game/JayCollab/FX/NS_SteamFX_System.NS_SteamFX_System")))

(event `self.ReceiveActorBeginOverlap`
  (params (OtherActor :type "Actor Object Reference"))
  (`parent.ReceiveActorBeginOverlap` OtherActor))

(event `self.ReceiveAnyDamage`
  (params (Damage :type "Float (single-precision)") (DamageType :type "DamageType Object Reference") (InstigatedBy :type "Controller Object Reference") (DamageCauser :type "Actor Object Reference"))
  (bind _frame (`self.Frame`))
  (bind _currentplatehealth (`self.CurrentPlateHealth`))
  ;[1 0.7919 0] Damage system for plate (will drop when food is cold or plate has 0 Health) (W.I.P)
  (set `self.CurrentPlateHealth` (- _currentplatehealth Damage))
  (if (<= _currentplatehealth 0.0)
    ;[1 0.7919 0] Customer will leave, points will be deducted, reset counter and delivery point
    (`/Engine/EditorBlueprintResources/StandardMacros.DoOnce` false :!label _label
      (:`Completed`
        (`/Game/AlexCollab/PickupSystem/BP_Counter.ClearCounter` (`self.Parent Counter`))
        (`/Game/AlexCollab/PickupSystem/BP_DeliveryPoint.F_DespawnPlate` (`self.Delivery Point`))
        (`|ExecutionSequence`
          (:`then_0`
            (bind _character (`self.Character`)
              (:`then`
                (set `/Game/JayCollab/BP_BaseCharacter.HasPlate` false _character)
                (`|SpawnActorFromClass` "/Game/JayCollab/Blueprints/CleanableHazards/BP_DroppedPlateHazard.BP_DroppedPlateHazard_C" (`SceneComponent.K2_GetComponentToWorld` (`/Game/JayCollab/BP_BaseCharacter.PlateDropLocation` _character)) "Undefined" "OverrideRootScale" null (struct :`R` 1.0 :`G` 0.966577 :`A` 1.0) null)
                (`/Game/JayCollab/BP_BaseCharacter.HUD_Hide Thought Bubble` (`self.Character`)))
              (:`else`
                _))
            (`self.SetActorHiddenInGame` true)
            (`/Game/AlexCollab/HUD_PlateFrame.DeliveryFinished` _frame)
            (`KismetSystemLibrary.Delay` 0.62)
            (`Widget.RemoveFromParent` _frame)
            (`self.K2_DestroyActor`))
          (:`then_1`
            (message `/Game/JayCollab/BPI_TableAndPointsSystem.I_ModifyPoints` (`self.Gamemode`) true (* (`self.DroppedPoints`) -1))))))))

(event `PlateIsCold`
  ;[1 0.7919 0] Damage system for plate (will drop when food is cold or plate has 0 Health) (W.I.P)
  (goto _label))

(fn `F_DropObject`
  (`parent.F_DropObject`)
  (`WidgetSwitcher.SetActiveWidgetIndex` (`/Game/AlexCollab/HUD_PlateFrame.IconState` (`self.Frame`)) 1))

(fn `F_PickUpObject`
  (bind _character (`self.Character`))
  (bind _frame (`self.Frame`))
  (`parent.F_PickUpObject`)
  (bind _parent_counter (`self.Parent Counter`)
    (:`then`
      (set `/Game/AlexCollab/PickupSystem/BP_Counter.PlateDocked` false _parent_counter)
      (`self.Character`
        (:`then`
          (`/Game/JayCollab/BP_BaseCharacter.Set Current Held Plate` _character self)
          (`/Game/AlexCollab/PickupSystem/BP_DeliveryPoint.Is Current Delivery Point` (`self.Delivery Point`) (`/Game/JayCollab/BP_BaseCharacter.CharacterColour` _character))
          (`WidgetSwitcher.SetActiveWidgetIndex` (`/Game/AlexCollab/HUD_PlateFrame.IconState` _frame) 2)
          (bind _returnvalue (`Image.GetDynamicMaterial` (`/Game/AlexCollab/HUD_PlateFrame.Image_1` _frame)))
          (`MaterialInstanceDynamic.SetTextureParameterValue` _returnvalue "RenderTexture" (`SceneCaptureComponent2D.TextureTarget` (`/Game/JayCollab/BP_BaseCharacter.SceneCaptureComponent2D` (`self.Character`)))))
        (:`else`)))
    (:`else`)))

(fn `F_SetPlateVariables`
  (set `self.CurrentPlateHealth` (`self.MaxPlateHealth`))
  (set `self.CurrentPlateQuality` (`self.StartingPlateQuality`)))

(fn `UserConstructionScript`
  (`parent.UserConstructionScript`))