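; BP_HelRiftMod is a rift hazard modifier that pulls on nearby characters and expires after ten seconds.
; A character (BPI_CharacterInput) entering HazardEffectArea receives an interface message and starts a fast looping timer that repeatedly fires RadialForce impulses.
; Leaving the area clears the timer, as does touching the Box trigger after a brief delay.
; Each pulse also draws a debug sphere at Centre.
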(event `self.ReceiveBeginPlay`
  (`parent.ReceiveBeginPlay`)
  (`self.SetLifeSpan` 10.0))

(event `self.HazardEffectArea.OnComponentBeginOverlap`
  (params (OverlappedComponent :type "PrimitiveComponent Object Reference") (OtherActor :type "Actor Object Reference") (OtherComp :type "PrimitiveComponent Object Reference") (OtherBodyIndex :type Integer) (bFromSweep :type Boolean) (SweepResult :type "HitResult Structure (by ref)"))
  (if (`KismetSystemLibrary.DoesImplementInterface` OtherActor "/Game/JayCollab/Interfaces/BPI_CharacterInput.BPI_CharacterInput_C")
    (message `/Game/JayCollab/Interfaces/BPI_CharacterInput.I_CurrentCharacter` OtherActor)
    (bind _returnvalue (`KismetSystemLibrary.K2_SetTimerDelegate` (delegate `PullingEvent`) 0.01 true))
    (set `self.LoopingForceHandle` _returnvalue)))

(event `PullingEvent`
  (`RadialForceComponent.FireImpulse` (`self.RadialForce`))
  (`KismetSystemLibrary.DrawDebugSphere` (`SceneComponent.K2_GetComponentLocation` (`self.Centre`)) 300.0 12 (struct :`G` 1.0 :`B` 0.665387 :`A` 1.0) 1.0 2.0))

(event `self.HazardEffectArea.OnComponentEndOverlap`
  (params (OverlappedComponent :type "PrimitiveComponent Object Reference") (OtherActor :type "Actor Object Reference") (OtherComp :type "PrimitiveComponent Object Reference") (OtherBodyIndex :type Integer))
  (if (`KismetSystemLibrary.DoesImplementInterface` OtherActor "/Game/JayCollab/Interfaces/BPI_CharacterInput.BPI_CharacterInput_C")
    (`KismetSystemLibrary.K2_ClearAndInvalidateTimerHandle` (`self.LoopingForceHandle`))))

(event `self.Box.OnComponentBeginOverlap`
  (params (OverlappedComponent :type "PrimitiveComponent Object Reference") (OtherActor :type "Actor Object Reference") (OtherComp :type "PrimitiveComponent Object Reference") (OtherBodyIndex :type Integer) (bFromSweep :type Boolean) (SweepResult :type "HitResult Structure (by ref)"))
  (if (`KismetSystemLibrary.DoesImplementInterface` OtherActor "/Game/JayCollab/Interfaces/BPI_CharacterInput.BPI_CharacterInput_C")
    (`KismetSystemLibrary.Delay` 0.06)
    (`KismetSystemLibrary.K2_ClearAndInvalidateTimerHandle` (`self.LoopingForceHandle`))))

(fn `UserConstructionScript`
  (`parent.UserConstructionScript`))