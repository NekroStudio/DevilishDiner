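; Dark Void modifier actor that drastically slows all players for a set duration while a post-process effect is active.
; Shortly after spawning, it messages every player in the game mode's list through interface calls to change movement speed, resetting it when time runs out.
; A runtime-added post-process component is blended in and out by looping timers.
; After blend-out, it destroys the component and, after a delay, itself.
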(event `self.ReceiveBeginPlay`
  ;[1 1 1] ActivateVoid when spawned
  (`parent.ReceiveBeginPlay`)
  (`KismetSystemLibrary.Delay` 0.5)
  (`self.ActivateVoid`))

(event `ActivateVoid`
  ;[1 1 1] Drastically slow movement speed for all players
  (`self.BlendPostProcess`)
  (for _array_element (`/Game/JayCollab/GM_DevilishDiner.AllPlayers` (`/Game/JayCollab/Interfaces/BPL_FunctionLib.F_GetGamemode`))
    (message `/Game/JayCollab/Blueprints/CleanableHazards/BPI_HazardsAndTools.I_TweakMovementSpeed` _array_element (`self.Move Speed`)))
  (`KismetSystemLibrary.Delay` (`self.Duration`))
  (`self.ResetVoid`))

(event `BlendPostProcess`
  ;[1 1 1] Blend Post Process
  (bind _returnvalue (`AddComponent|NODE_AddPostProcessComponent-0` :`bManualAttachment` true :`RelativeTransform` (`self.GetTransform`)))
  (set `self.PostProcess` _returnvalue)
  (bind _returnvalue_2 (`KismetSystemLibrary.K2_SetTimerDelegate` (delegate `EventBlendIncrease`) 0.01 true))
  (set `self.BlendLoopHandle` _returnvalue_2))

(event `EventBlendIncrease`
  ;[1 1 1] Blend Post Process
  (bind _blendweight (`PostProcessComponent.BlendWeight` (stale `BlendPostProcess` _returnvalue)))
  (set `PostProcessComponent.BlendWeight` (+ _blendweight (`self.BlendChange`)) (stale `BlendPostProcess` _returnvalue))
  (if (>= _blendweight 1.0)
    (`KismetSystemLibrary.K2_ClearAndInvalidateTimerHandle` (`self.BlendLoopHandle`))))

(event `ResetVoid`
  ;[1 1 1] Reset movement speed
  (for _array_element (`/Game/JayCollab/GM_DevilishDiner.AllPlayers` (`/Game/JayCollab/Interfaces/BPL_FunctionLib.F_GetGamemode`))
    (message `/Game/JayCollab/Blueprints/CleanableHazards/BPI_HazardsAndTools.I_ResetMovementSpeed` _array_element))
  (`self.UnblendPostProcess`))

(event `UnblendPostProcess`
  ;[1 1 1] UnblendPostProcess
  (bind _returnvalue (`KismetSystemLibrary.K2_SetTimerDelegate` (delegate `EventBlendDecrease`) 0.01 true))
  (set `self.UnblendLoopHandle` _returnvalue))

(event `EventBlendDecrease`
  (bind _postprocess (`self.PostProcess`))
  (bind _blendweight (`PostProcessComponent.BlendWeight` _postprocess))
  ;[1 1 1] UnblendPostProcess
  (set `PostProcessComponent.BlendWeight` (- _blendweight (`self.BlendChange`)) _postprocess)
  (if (<= _blendweight 0.0)
    (`KismetSystemLibrary.K2_ClearAndInvalidateTimerHandle` (`self.UnblendLoopHandle`))
    (`ActorComponent.K2_DestroyComponent` _postprocess)
    (`KismetSystemLibrary.Delay` 3.0)
    (`self.K2_DestroyActor`)))

(fn `UserConstructionScript`
  (`parent.UserConstructionScript`))