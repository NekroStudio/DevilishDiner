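; Corrupted Blood modifier: a short-lived hazard area that spreads corruption to characters and damages the plate they hold.
; On overlap, a DoOnce-gated path messages the character through interface calls, then starts looping timer damage on any held plate, pauses its quality and adds FX.
; Leaving clears the timer immediately and re-arms entry, then after a delay removes FX, resumes plate quality and stops the spread.
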(event `self.ReceiveBeginPlay`
  ;[1 1 1] Begin play
  (`parent.ReceiveBeginPlay`)
  (`self.SetLifeSpan` 10.0))

(event `self.HazardEffectArea.OnComponentBeginOverlap`
  (params (OverlappedComponent :type "PrimitiveComponent Object Reference") (OtherActor :type "Actor Object Reference") (OtherComp :type "PrimitiveComponent Object Reference") (OtherBodyIndex :type Integer) (bFromSweep :type Boolean) (SweepResult :type "HitResult Structure (by ref)"))
  (bind _held_plate_ref (`self.Held Plate Ref`))
  ;[1 1 1] Damage overlap if in hazard
  (if (`KismetSystemLibrary.DoesImplementInterface` OtherActor "/Game/JayCollab/Interfaces/BPI_CharacterInput.BPI_CharacterInput_C")
    (`/Engine/EditorBlueprintResources/StandardMacros.DoOnce` false :!label _label
      (:`Completed`
        (bind _heldplate (message `/Game/JayCollab/Blueprints/CleanableHazards/BPI_HazardsAndTools.I_CurrentHeldPlate` OtherActor))
        (set `self.Held Plate Ref` _heldplate)
        (`/Engine/EditorBlueprintResources/StandardMacros.IsValid` _heldplate
          (:`Is Valid`
            (message `/Game/JayCollab/Blueprints/CleanableHazards/BPI_HazardsAndTools.I_SpreadCorruptedBlood` OtherActor)
            (`|ExecutionSequence`
              (:`then_0`
                (bind _returnvalue (`KismetSystemLibrary.K2_SetTimerDelegate` (delegate `DamagePlate`) (`self.DamageLoopTime`) true :!label _label_2))
                (set `self.DamageLoopHandle` _returnvalue)
                (`/Engine/EditorBlueprintResources/StandardMacros.IsValid` _held_plate_ref
                  (:`Is Valid`
                    (message `/Game/JayCollab/Interfaces/BPI_PlateCommunication.I_PausePlateQuality` _held_plate_ref))))
              (:`then_1`
                (`/Game/AlexCollab/PickupSystem/BP_Plate.CorruptedBloodFx` (`self.Held Plate Ref`) self)
                (`self.ResetDoOnceEndOverlap`))))
          (:`Is Not Valid`
            (message `/Game/JayCollab/Blueprints/CleanableHazards/BPI_HazardsAndTools.I_SpreadCorruptedBlood` OtherActor)))))))

(event `StartDamageLoop`
  ;[1 1 1] Damage overlap if in hazard
  (goto _label_2))

(event `DamagePlate`
  ;[1 1 1] Damage overlap if in hazard
  (`GameplayStatics.ApplyDamage` (`self.Held Plate Ref`) (`self.Damage`) null self))

(event `self.HazardEffectArea.OnComponentEndOverlap`
  (params (OverlappedComponent :type "PrimitiveComponent Object Reference") (OtherActor :type "Actor Object Reference") (OtherComp :type "PrimitiveComponent Object Reference") (OtherBodyIndex :type Integer))
  ;[1 1 1] Leave damage volume
  (if (`KismetSystemLibrary.DoesImplementInterface` OtherActor "/Game/JayCollab/Interfaces/BPI_CharacterInput.BPI_CharacterInput_C")
    (`|ExecutionSequence`
      (:`then_0`
        (`KismetSystemLibrary.K2_ClearAndInvalidateTimerHandle` (`self.DamageLoopHandle`))
        (`KismetSystemLibrary.Delay` (`self.EndOverlapDamageDelay`))
        (`/Engine/EditorBlueprintResources/StandardMacros.DoOnce` false :!label _label_3
          (:`Completed`
            (bind _held_plate_ref (`self.Held Plate Ref`)
              (:`then`
                (`/Game/AlexCollab/PickupSystem/BP_Plate.RemoveCorruptedBloodFx` _held_plate_ref self)
                (message `/Game/JayCollab/Interfaces/BPI_PlateCommunication.I_ResumePlateQuality` _held_plate_ref))
              (:`else`
                _))
            (message `/Game/JayCollab/Blueprints/CleanableHazards/BPI_HazardsAndTools.I_StopSpreadCorruptedBlood` OtherActor))))
      (:`then_1`
        (goto _label :!via `Reset`)))))

(event `ResetDoOnceEndOverlap`
  ;[1 1 1] Leave damage volume
  (goto _label_3 :!via `Reset`))

(fn `UserConstructionScript`
  (`parent.UserConstructionScript`))