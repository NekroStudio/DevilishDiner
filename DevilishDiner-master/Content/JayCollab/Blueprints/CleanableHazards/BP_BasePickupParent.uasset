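; Base pickup actor, in the CleanableHazards folder, that rotates its Scene component and notifies overlapping characters of an available tool.
; On begin overlap, actors implementing BPI_CharacterInput receive IPickedUpToolMessage with the pickup itself, both immediately and again from a short one-shot timer.
; On end overlap, it cancels that timer and sends the same message with an empty reference.
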(event `self.ReceiveBeginPlay`
  (`parent.ReceiveBeginPlay`)
  (`MovementComponent.SetUpdatedComponent` (`self.RotatingMovement`) (`self.Scene`)))

(event `self.Collision.OnComponentBeginOverlap`
  (params (OverlappedComponent :type "PrimitiveComponent Object Reference") (OtherActor :type "Actor Object Reference") (OtherComp :type "PrimitiveComponent Object Reference") (OtherBodyIndex :type Integer) (bFromSweep :type Boolean) (SweepResult :type "HitResult Structure (by ref)"))
  (if (`KismetSystemLibrary.DoesImplementInterface` OtherActor "/Game/JayCollab/Interfaces/BPI_CharacterInput.BPI_CharacterInput_C")
    (bind _returnvalue (`KismetSystemLibrary.K2_SetTimerDelegate` (delegate `PickedUpTool`) 0.2))
    (set `self.Handle` _returnvalue)
    (message `/Game/JayCollab/Blueprints/CleanableHazards/BPI_HazardsAndTools.I_PickedUpTool` OtherActor self :!label _label)))

(event `PickedUpTool`
  (goto _label))

(event `self.Collision.OnComponentEndOverlap`
  (params (OverlappedComponent :type "PrimitiveComponent Object Reference") (OtherActor :type "Actor Object Reference") (OtherComp :type "PrimitiveComponent Object Reference") (OtherBodyIndex :type Integer))
  (if (`KismetSystemLibrary.DoesImplementInterface` OtherActor "/Game/JayCollab/Interfaces/BPI_CharacterInput.BPI_CharacterInput_C")
    (`KismetSystemLibrary.K2_ClearAndInvalidateTimerHandle` (`self.Handle`))
    (message `/Game/JayCollab/Blueprints/CleanableHazards/BPI_HazardsAndTools.I_PickedUpTool` OtherActor null)))

(fn `UserConstructionScript`
  (`parent.UserConstructionScript`))