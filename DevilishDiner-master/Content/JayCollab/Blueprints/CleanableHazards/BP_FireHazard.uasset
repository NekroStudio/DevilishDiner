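; BP_FireHazard is a fire hazard that damages the plate held by an actor inside its effect area.
; On overlap begin, it gets the held plate through an interface call and, if valid, starts a looping one-second timer that applies the Damage value to that plate.
; Any end overlap on the area clears the timer, without checking which actor left.
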(event `self.HazardEffectArea.OnComponentBeginOverlap`
  (params (OverlappedComponent :type "PrimitiveComponent Object Reference") (OtherActor :type "Actor Object Reference") (OtherComp :type "PrimitiveComponent Object Reference") (OtherBodyIndex :type Integer) (bFromSweep :type Boolean) (SweepResult :type "HitResult Structure (by ref)"))
  (bind _heldplate (message `/Game/JayCollab/Blueprints/CleanableHazards/BPI_HazardsAndTools.I_CurrentHeldPlate` OtherActor))
  (`/Engine/EditorBlueprintResources/StandardMacros.IsValid` _heldplate
    (:`Is Valid`
      (bind _returnvalue (`KismetSystemLibrary.K2_SetTimerDelegate` (delegate `DamagePlate`) 1.0 true))
      (set `self.DamageLoopHandle` _returnvalue))))

(event `DamagePlate`
  (`GameplayStatics.ApplyDamage` (stale `self.HazardEffectArea.OnComponentBeginOverlap` _heldplate) (`self.Damage`) null self))

(event `self.HazardEffectArea.OnComponentEndOverlap`
  (params (OverlappedComponent :type "PrimitiveComponent Object Reference") (OtherActor :type "Actor Object Reference") (OtherComp :type "PrimitiveComponent Object Reference") (OtherBodyIndex :type Integer))
  (`KismetSystemLibrary.K2_ClearAndInvalidateTimerHandle` (`self.DamageLoopHandle`)))

(fn `UserConstructionScript`
  (`parent.UserConstructionScript`))