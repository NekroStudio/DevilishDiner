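; Ectoplasm hazard, filed among the cleanable hazards, that slows characters while they stand in its effect area.
; On begin play it applies its configured colour.
; Overlaps on the HazardEffectArea component send a speed impairment to actors implementing BPI_CharacterInput and a reset when they leave, so it needs no character cast.
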(event `self.ReceiveBeginPlay`
  (`parent.ReceiveBeginPlay`)
  (`self.Set Colour` (`self.Colour`)))

(event `self.HazardEffectArea.OnComponentBeginOverlap`
  (params (OverlappedComponent :type "PrimitiveComponent Object Reference") (OtherActor :type "Actor Object Reference") (OtherComp :type "PrimitiveComponent Object Reference") (OtherBodyIndex :type Integer) (bFromSweep :type Boolean) (SweepResult :type "HitResult Structure (by ref)"))
  (if (`KismetSystemLibrary.DoesImplementInterface` OtherActor "/Game/JayCollab/Interfaces/BPI_CharacterInput.BPI_CharacterInput_C")
    (message `/Game/JayCollab/Blueprints/CleanableHazards/BPI_HazardsAndTools.I_TweakMovementSpeed` OtherActor (`self.SpeedImpairment`))))

(event `self.HazardEffectArea.OnComponentEndOverlap`
  (params (OverlappedComponent :type "PrimitiveComponent Object Reference") (OtherActor :type "Actor Object Reference") (OtherComp :type "PrimitiveComponent Object Reference") (OtherBodyIndex :type Integer))
  (if (`KismetSystemLibrary.DoesImplementInterface` OtherActor "/Game/JayCollab/Interfaces/BPI_CharacterInput.BPI_CharacterInput_C")
    (message `/Game/JayCollab/Blueprints/CleanableHazards/BPI_HazardsAndTools.I_ResetMovementSpeed` OtherActor)))

(fn `UserConstructionScript`
  (`parent.UserConstructionScript`))