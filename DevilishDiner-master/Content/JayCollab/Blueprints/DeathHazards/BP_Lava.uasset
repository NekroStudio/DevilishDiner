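; BP_Lava is a lava death hazard that triggers on overlap with actors implementing BPI_CharacterInput.
; It sends the player death message with a duration, stops their movement and hides them, leaving respawn and unhiding to code outside this Blueprint.
; A macro then degrades the quality of any plate the player holds.
; The random player-start teleport macro holds only unused logic.
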(event `self.Collision.OnComponentBeginOverlap`
  (params (OverlappedComponent :type "PrimitiveComponent Object Reference") (OtherActor :type "Actor Object Reference") (OtherComp :type "PrimitiveComponent Object Reference") (OtherBodyIndex :type Integer) (bFromSweep :type Boolean) (SweepResult :type "HitResult Structure (by ref)"))
  ;[1 1 1] Respawn player at a player start location, stop movement and temporarily set to hidden. Undo these features when respawning
  (if (`KismetSystemLibrary.DoesImplementInterface` OtherActor "/Game/JayCollab/Interfaces/BPI_CharacterInput.BPI_CharacterInput_C")
    (`|ExecutionSequence`
      (:`then_0`
        (message `/Game/JayCollab/Interfaces/BPI_CharDeath.I_PlayerDeath` OtherActor (`self.DeathDuration`))
        (message `/Game/JayCollab/Interfaces/BPI_CharacterInput.I_StopMovement` OtherActor)
        (`self.SetActorHiddenInGame` OtherActor true))
      (:`then_1`
        (`/Engine/EditorBlueprintResources/StandardMacros.IsValid` OtherActor
          (:`Is Valid`
            (`self.M_RemovePlate` OtherActor)))))))

(fn `UserConstructionScript`
  (`parent.UserConstructionScript`))