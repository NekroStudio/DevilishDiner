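; BP_TableLocation is a table trigger volume that tracks how many customers occupy it, up to a maximum capacity.
; Box overlaps raise or lower the count without filtering the overlapping actor, flagging the table full when an overlap begins at capacity.
; Count changes are sent to the game mode by interface message, and an interface function returns the current count.
; The construction script sizes the box from a variable.
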(event `self.TableLocation.OnComponentBeginOverlap`
  (params (OverlappedComponent :type "PrimitiveComponent Object Reference") (OtherActor :type "Actor Object Reference") (OtherComp :type "PrimitiveComponent Object Reference") (OtherBodyIndex :type Integer) (bFromSweep :type Boolean) (SweepResult :type "HitResult Structure (by ref)"))
  (bind _currenttablecapacity (`self.CurrentTableCapacity`))
  (if (== _currenttablecapacity (`self.MaxTableCapacity`))
    (set `self.TableIsFull` true)
    (`KismetSystemLibrary.PrintString` "TABLEFULL" true true (struct :`R` 1.0 :`B` 0.002792 :`A` 1.0))
    (else
      (`/Engine/EditorBlueprintResources/StandardMacros.IncrementInt` _currenttablecapacity
        (:`  `
          (message `/Game/JayCollab/BPI_TableAndPointsSystem.I_UpdateTableCustomers` (`GameplayStatics.GetGameMode`) (`self.CurrentTableCapacity`)))))))

(event `self.TableLocation.OnComponentEndOverlap`
  (params (OverlappedComponent :type "PrimitiveComponent Object Reference") (OtherActor :type "Actor Object Reference") (OtherComp :type "PrimitiveComponent Object Reference") (OtherBodyIndex :type Integer))
  (`/Engine/EditorBlueprintResources/StandardMacros.DecrementInt` (`self.CurrentTableCapacity`)
    (:`  `
      (set `self.TableIsFull` false)
      (message `/Game/JayCollab/BPI_TableAndPointsSystem.I_UpdateTableCustomers` (`GameplayStatics.GetGameMode`) (`self.CurrentTableCapacity`)))))

(fn `I_CurrentTableCustomers`
  (returns (TableCustomers :type Integer))
  (return (`self.CurrentTableCapacity`)))

(fn `UserConstructionScript`
  (`BoxComponent.SetBoxExtent` (`self.TableLocation`) (`self.In Box Extent`) true))