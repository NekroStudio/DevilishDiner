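; BP_ChairLocation marks a seating spot at a table and tracks whether it is occupied.
; A box collider named TableLocation, sized in the construction script, sets ChairsFull when an overlap begins and clears it when one ends, printing debug messages.
; An interface function returns CurrentTableCapacity to callers, though this graph never updates that value.
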(event `self.TableLocation.OnComponentBeginOverlap`
  (params (OverlappedComponent :type "PrimitiveComponent Object Reference") (OtherActor :type "Actor Object Reference") (OtherComp :type "PrimitiveComponent Object Reference") (OtherBodyIndex :type Integer) (bFromSweep :type Boolean) (SweepResult :type "HitResult Structure (by ref)"))
  (set `self.ChairsFull` true)
  (`KismetSystemLibrary.PrintString` "TABLEFULL" true true (struct :`R` 1.0 :`B` 0.002792 :`A` 1.0)))

(event `self.TableLocation.OnComponentEndOverlap`
  (params (OverlappedComponent :type "PrimitiveComponent Object Reference") (OtherActor :type "Actor Object Reference") (OtherComp :type "PrimitiveComponent Object Reference") (OtherBodyIndex :type Integer))
  (set `self.ChairsFull` false)
  (`KismetSystemLibrary.PrintString` "TABLEEMPTY" true true (struct :`R` 1.0 :`B` 0.002792 :`A` 1.0)))

(fn `I_CurrentTableCustomers`
  (returns (TableCustomers :type Integer))
  (return (`self.CurrentTableCapacity`)))

(fn `UserConstructionScript`
  (`BoxComponent.SetBoxExtent` (`self.TableLocation`) (`self.In Box Extent`) true))