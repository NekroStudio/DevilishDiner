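; BP_PointsVolume is a one-shot trigger volume that changes the points in Devilish Diner when a player enters it.
; On BeginPlay it caches the GM_DevilishDiner game mode, and the construction script sizes its box from an exposed extent.
; A player overlap sends the configured point amount and positive-or-negative flag to the game mode by interface message, then destroys the volume.
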(event `self.ReceiveBeginPlay`
  (bind _asgm_devilish_diner (cast `/Game/JayCollab/GM_DevilishDiner` (`GameplayStatics.GetGameMode`)))
  (set `self.Gamemode` _asgm_devilish_diner))

(event `self.Box.OnComponentBeginOverlap`
  (params (OverlappedComponent :type "PrimitiveComponent Object Reference") (OtherActor :type "Actor Object Reference") (OtherComp :type "PrimitiveComponent Object Reference") (OtherBodyIndex :type Integer) (bFromSweep :type Boolean) (SweepResult :type "HitResult Structure (by ref)"))
  (`/Game/JayCollab/BP_MacroLibrary.IsPlayer?` OtherActor
    (:`IsPlayer`
      (message `/Game/JayCollab/BPI_PointsSystem.I_ModifyPoints` (`self.Gamemode`) (`self.Positive Modification`) (`self.PointsModified`))
      (`self.K2_DestroyActor`))))

(fn `UserConstructionScript`
  (`BoxComponent.SetBoxExtent` (`self.Box`) (`self.BoxExtent`) true))