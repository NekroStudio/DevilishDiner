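; BP_ChairLocation is a configurable chair that seats customers and reports whether it is occupied.
; Overlapping the seat box marks it full and, once per occupancy, snaps customers not tagged LeavingCustomer to the sit point and arrow rotation.
; A further overlap while full disables seat collision; end overlap or a customer exit interface call frees and re-enables it.
; The construction script sets box size, chair scale, collision and enabled state.
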(event `/Game/JayCollab/Blueprints/ChairLocations/BPI_CustomerTableInfo.I_ChairFull`
  (set `self.ChairIsFull` true))

(event `/Game/JayCollab/Blueprints/ChairLocations/BPI_CustomerTableInfo.I_ChairEmpty`
  (set `self.ChairIsFull` false))

(event `self.SeatLocation.OnComponentBeginOverlap`
  (params (OverlappedComponent :type "PrimitiveComponent Object Reference") (OtherActor :type "Actor Object Reference") (OtherComp :type "PrimitiveComponent Object Reference") (OtherBodyIndex :type Integer) (bFromSweep :type Boolean) (SweepResult :type "HitResult Structure (by ref)"))
  (if (`self.ChairIsFull`)
    (`self.F_DisableSeat`)
    (else
      (set `self.ChairIsFull` true)
      (bind _customer (message `/Game/MathieuLecerfCollab/AnimationFolder/AnimationFolder/BPI_CustomerAnimations.I_GetCustomer` OtherActor))
      (set `self.CurrentCustomer` _customer)
      (if (not (`self.ActorHasTag` _customer "LeavingCustomer"))
        (`/Engine/EditorBlueprintResources/StandardMacros.DoOnce` false :!label _label
          (:`Completed`
            (`self.K2_SetActorTransform` (`self.CurrentCustomer`) (`KismetMathLibrary.MakeTransform` (`SceneComponent.K2_GetComponentLocation` (`self.SitLocation`)) (`SceneComponent.K2_GetComponentRotation` (`self.Arrow`))) false false)))))))

(event `ResetDoOnce`
  (goto _label :!via `Reset`))

(event `self.SeatLocation.OnComponentEndOverlap`
  (params (OverlappedComponent :type "PrimitiveComponent Object Reference") (OtherActor :type "Actor Object Reference") (OtherComp :type "PrimitiveComponent Object Reference") (OtherBodyIndex :type Integer))
  ;[1 1 1] End overlap, leave seat and reset chair is full
  (set `self.ChairIsFull` false :!label _label_2)
  (`self.F_EnableSeat`)
  (`self.ResetDoOnce`))

(event `/Game/JayCollab/Blueprints/ChairLocations/BPI_CustomerTableInfo.I_CustomerExit`
  ;[1 1 1] End overlap, leave seat and reset chair is full
  (bind _currentcustomer (`self.CurrentCustomer`)
    (:`then`
      (message `/Game/JayCollab/AI/BPI_CustomerInterface.I_MessageCustomerExit` _currentcustomer)
      (goto _label_2))
    (:`else`)))

(fn `F_DisableSeat`
  (`PrimitiveComponent.SetCollisionEnabled` (`self.SeatLocation`) "NoCollision"))

(fn `F_EnableSeat`
  (`PrimitiveComponent.SetCollisionEnabled` (`self.SeatLocation`) "QueryAndPhysics"))

(fn `I_GetChairStatus`
  (returns (ChairIsFull :type Boolean))
  (return (`self.ChairIsFull`)))

(fn `UserConstructionScript`
  (bind _seatlocation (`self.SeatLocation`))
  (bind _seatlocation_2 (`self.SeatLocation`))
  (bind _chair (`self.Chair`))
  (`BoxComponent.SetBoxExtent` (`self.SeatLocation`) (`self.In Box Extent`) true)
  (`SceneComponent.SetWorldScale3D` (`self.Chair`) (`self.ChairSize`))
  (if (`self.IsEnabled`)
    (`PrimitiveComponent.SetCollisionEnabled` _seatlocation "QueryAndPhysics")
    (set `self.ChairIsFull` false)
    (`SceneComponent.SetVisibility` _seatlocation_2 true false)
    (else
      (`PrimitiveComponent.SetCollisionEnabled` _seatlocation "NoCollision")
      (set `self.ChairIsFull` true)
      (`SceneComponent.SetVisibility` _seatlocation_2 false false)))
  (if (`self.EnableChairCollision`)
    (`PrimitiveComponent.SetCollisionEnabled` _chair "QueryAndPhysics")
    (else
      (`PrimitiveComponent.SetCollisionEnabled` _chair "NoCollision"))))