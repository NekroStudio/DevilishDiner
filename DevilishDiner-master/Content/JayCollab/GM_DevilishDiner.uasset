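; Game mode for Devilish Diner, a timed local co-op diner game for up to four players sharing a team score.
; BeginPlay spawns color-coded players at tagged starts, freezing movement until the HUD countdown ends.
; A randomly re-armed timer spawns customers and PlateManager deliveries for free counters, stopping at last orders.
; Point changes and clock ticks broadcast through dispatchers, and time-out compares the score to a target for win or lose.
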(event `self.ReceiveBeginPlay`
  ;[1 1 1] Begin play - Init chain (before game starts)
  (`self.F_InitGameInstanceVars`)
  (`self.F_GetPlayerStartPoints`)
  (`self.F_SpawnAllPlayers`)
  (`self.F_ChangeAllPlayerMovement` "MOVE_None")
  (`self.F_InitHUD`)
  (`/Game/JayCollab/BP_Camera.InitCamera` (`self.GlobalCamera`))
  (`self.F_GetCustomerSpawnLocations`)
  (`/Game/AlexCollab/HUD_StartingTimerCountdown.FireTimerCountdown` (`/Game/AlexCollab/HUD_Manager.HUD_StartingTimerCountdown` (`self.HUD`)))
  (`self.F_HideMouseCursors`))

(event `/Game/JayCollab/BPI_HUDEvents.I_CountdownTimerFin`
  ;[1 1 1] After initial timer countdown finishes (after game starts)
  (`self.F_ChangeAllPlayerMovement` "MOVE_Walking")
  (`self.StartGameTimer`)
  (`/Game/AlexCollab/HUD_Manager.ShrinkTimeEvent` (`self.HUD`))
  (`self.Trigger Deliveries Spawning`))

(event `/Game/JayCollab/BPI_TableAndPointsSystem.I_ModifyPoints`
  (params (PositiveModification :type Boolean) (Points :type Integer))
  ;[1 1 1] Points System
  (bind _currentpoints (`self.F_PointsModificationSystem` PositiveModification Points))
  (`self.ED_UpdatePoints` _currentpoints))

(event `Star rating system`
  ;[1 1 1] Win Lose and Star Conditions
)

(event `Win Condition`
  ;[1 1 1] Win Lose and Star Conditions
  (`/Game/AlexCollab/HUD_EndCondition.EndConditionText` (`/Game/AlexCollab/HUD_Manager.HUD_EndCondition` (`self.HUD`)) "You Win!" (struct :`R` 0.004252 :`G` 1.0 :`A` 1.0) (`self.CurrentTeamPoints`)))

(event `StartGameTimer`
  ;[1 0.9555 0] Gameplay Start Timer (W.I.P)
  (bind _returnvalue (`KismetSystemLibrary.K2_SetTimerDelegate` (delegate `GameplayTimerEvent`) (`self.LoopingFloatForTimer`) true))
  (set `self.GameplayDurationHandle` _returnvalue))

(event `GameplayTimerEvent`
  (bind _gameplaytimeduration (`self.GameplayTimeDuration`))
  (bind _hud_startingtimercountdown (`/Game/AlexCollab/HUD_Manager.HUD_StartingTimerCountdown` (`self.HUD`)))
  ;[1 0.9555 0] Gameplay Start Timer (W.I.P)
  (`UserWidget.PlayAnimation` _hud_startingtimercountdown (`/Game/AlexCollab/HUD_StartingTimerCountdown.TickOver` _hud_startingtimercountdown) 0.0 1 "Forward" 1.0 false)
  (`KismetSystemLibrary.Delay` 0.25)
  (if (<= _gameplaytimeduration 15.0)
    (`self.Opening/ClosingTime`))
  (bind _result (`/Engine/EditorBlueprintResources/StandardMacros.DecrementFloat` _gameplaytimeduration)
    (:`  `
      (`self.ED_TimeUpdated` _result)
      (if (<= _gameplaytimeduration 0.0)
        (`KismetSystemLibrary.K2_ClearAndInvalidateTimerHandle` (`self.GameplayDurationHandle`))
        (`/Game/AlexCollab/HUD_Manager.MatchFinished` (`self.HUD`))
        (if (>= (`self.CurrentTeamPoints`) (`self.PointsNeededToWin`))
          (`self.Win Condition`)
          (else
            (`self.Lose Condition`)))))))

(event `Lose Condition`
  ;[1 1 1] Win Lose and Star Conditions
  (`/Game/AlexCollab/HUD_EndCondition.EndConditionText` (`/Game/AlexCollab/HUD_Manager.HUD_EndCondition` (`self.HUD`)) "You Lose!" (struct :`R` 1.0 :`A` 1.0) (`self.CurrentTeamPoints`)))

(event `Opening/ClosingTime`
  ;[1 1 1] Opening/ClosingTime (stop customers entering
  (`/Engine/EditorBlueprintResources/StandardMacros.DoOnce` false
    (:`Completed`
      (`KismetSystemLibrary.PrintString` "Last Orders!" true true (struct :`R` 1.0 :`B` 0.338718 :`A` 1.0))
      (`KismetSystemLibrary.K2_ClearAndInvalidateTimerHandle` (`self.CustomerSpawnLoopHandle`)))))

(event `Trigger Deliveries Spawning`
  ;[1 1 1] Spawn Customers
  (set `self.MaxNumberOfChairs` (`KismetArrayLibrary.Array_Length` (`/Game/AlexCollab/PickupSystem/BP_PlateManager.Delivery Points` (`self.PlateManager`))))
  (bind _returnvalue (`KismetSystemLibrary.K2_SetTimerDelegate` (delegate `EventDeliverySpawnLoop`) (`KismetMathLibrary.RandomFloatInRange` (`self.Looping Duration Min`) (`self.Looping Duration Max`)) true))
  (set `self.CustomerSpawnLoopHandle` _returnvalue))

(event `EventDeliverySpawnLoop`
  ;[1 1 1] Spawn Customers
  (bind _currentcounter (`self.F_CheckPlateDocked`))
  (bind _output_get (set `self.CurrentCounterVar` _currentcounter))
  (`/Engine/EditorBlueprintResources/StandardMacros.IsValid` _output_get
    (:`Is Valid`
      (if (<= (`self.NumOfCurrentChair`) (`self.MaxNumberOfChairs`))
        (`|SpawnActorFromClass` "/Game/JayCollab/AI/BP_Customer.BP_Customer_C" (`self.F_RandomCustomerSpawnLoc`) "Undefined" "OverrideRootScale" null null)
        (bind _delivery_point_to_be_assigned (`/Game/AlexCollab/PickupSystem/BP_PlateManager.Create Delivery` (`self.PlateManager`) (`self.CurrentCounterVar`)))
        (set `self.Linked Chair` (`/Game/AlexCollab/PickupSystem/BP_DeliveryPoint.LinkedChair` _delivery_point_to_be_assigned))
        (`/Engine/EditorBlueprintResources/StandardMacros.IncrementInt` (`self.NumOfCurrentChair`)
          (:`  `
            (`KismetSystemLibrary.K2_ClearAndInvalidateTimerHandle` (`self.CustomerSpawnLoopHandle`) :!label _label)
            (`KismetSystemLibrary.Delay` 0.25)
            (`self.Trigger Deliveries Spawning`)))))
    (:`Is Not Valid`
      (goto _label))))

(event `/Game/JayCollab/BPI_TableAndPointsSystem.I_DecreaseChairAmount`
  ;[1 1 1] Decrease Chair Amount
  (`/Engine/EditorBlueprintResources/StandardMacros.DecrementInt` (`self.NumOfCurrentChair`)))

(fn `F_ChangeAllPlayerMovement`
  (params (SetMovement :type "EMovementMode Enum" :default "MOVE_None"))
  (for _array_element (`self.AllPlayers`)
    (`CharacterMovementComponent.SetMovementMode` (`Character.CharacterMovement` _array_element) SetMovement 0)))

(fn `F_CheckPlateDocked`
  (returns (CurrentCounter :type "/Game/AlexCollab/PickupSystem/BP_Counter Object Reference"))
  (for _array_element (`self.AllCounters`)
    (if (not (`/Game/AlexCollab/PickupSystem/BP_Counter.PlateDocked` _array_element))
      (return _array_element)))
  (return null))

(fn `F_GetCustomerSpawnLocations`
  (bind _outactors (`GameplayStatics.GetAllActorsOfClass` "/Game/JayCollab/AI/BP_CustomerSpawnLocations.BP_CustomerSpawnLocations_C"))
  (set `self.AllChairSpawnLocations` _outactors))

(fn `F_GetPlayerStartPoints`
  (bind _outactors (`GameplayStatics.GetAllActorsOfClass` "/Script/Engine.PlayerStart"))
  (set `self.AllPlayerStarts` _outactors)
  (bind _outactors_2 (`GameplayStatics.GetAllActorsOfClass` "/Game/AlexCollab/PickupSystem/BP_PlateManager.BP_PlateManager_C"))
  (set `self.PlateManager` (`|GetArrayItem` _outactors_2))
  (bind _outactors_3 (`GameplayStatics.GetAllActorsOfClass` "/Game/JayCollab/BP_Camera.BP_Camera_C"))
  (set `self.GlobalCamera` (`|GetArrayItem` _outactors_3))
  (bind _outactors_4 (`GameplayStatics.GetAllActorsOfClass` "/Game/AlexCollab/PickupSystem/BP_Counter.BP_Counter_C"))
  (for _array_element _outactors_4
    (`KismetArrayLibrary.Array_AddUnique` (`self.AllCounters`) _array_element)))

(fn `F_HideMouseCursors`
  (for _array_element (`self.AllControllers`)
    (set `PlayerController.bShowMouseCursor` false _array_element)))

(fn `F_InitGameInstanceVars`
  (bind _asbp_game_instance (cast `/Game/JayCollab/BP_GameInstance` (`GameplayStatics.GetGameInstance`)))
  (bind _output_get (set `self.GameInstance` _asbp_game_instance))
  (set `self.MaxPlayerNumber` (`/Game/JayCollab/BP_GameInstance.PlayerCount` _output_get)))

(fn `F_InitHUD`
  (bind _returnvalue (`|CreateWidget` "/Game/AlexCollab/HUD_Manager.HUD_Manager_C"))
  (set `self.HUD` _returnvalue)
  (`UserWidget.AddToViewport` _returnvalue 0)
  (`/Game/AlexCollab/HUD_Manager.Init` _returnvalue (`self.AllPlayers`) self))

(fn `F_PointsModificationSystem`
  (params (Modification :type Boolean) (PointsIn :type Integer))
  (returns (CurrentPoints :type Integer))
  (if Modification
    (bind _output_get (set `self.CurrentTeamPoints` (+ (`self.CurrentTeamPoints`) PointsIn)))
    (return _output_get)
    (else
      (bind _output_get_2 (set `self.CurrentTeamPoints` (+ (`self.CurrentTeamPoints`) (* PointsIn -1))))
      (return _output_get_2))))

(fn `F_RandomCustomerSpawnLoc`
  (returns (RandomSpawnTrans :type "Transform Structure (by ref)"))
  (bind _allchairspawnlocations (`self.AllChairSpawnLocations`))
  (return (`self.GetTransform` (`|GetArrayItem` _allchairspawnlocations (`KismetMathLibrary.RandomIntegerInRange` 0 (- (`KismetArrayLibrary.Array_Length` _allchairspawnlocations) 1))))))

(fn `F_SetPlayerColour`
  (params (Character :type "/Game/JayCollab/BP_BaseCharacter Object Reference"))
  (bind _playerindex (`self.PlayerIndex`))
  (if (== _playerindex 0)
    (message `/Game/JayCollab/BPI_CharacterInput.I_CharacterColour` Character (struct :`R` 1.0 :`A` 1.0) "/Game/JayCollab/Materials/M_Male_BodyRed.M_Male_BodyRed")
    (elif (== _playerindex 1)
      (message `/Game/JayCollab/BPI_CharacterInput.I_CharacterColour` Character (struct :`B` 1.0 :`A` 1.0) "/Game/JayCollab/Materials/M_Male_BodyBlue.M_Male_BodyBlue")
      (elif (== _playerindex 2)
        (message `/Game/JayCollab/BPI_CharacterInput.I_CharacterColour` Character (struct :`G` 1.0 :`A` 1.0) "/Game/JayCollab/Materials/M_Male_BodyGreen1.M_Male_BodyGreen1")
        (elif (== _playerindex 3)
          (message `/Game/JayCollab/BPI_CharacterInput.I_CharacterColour` Character (struct :`R` 1.0 :`G` 1.0 :`A` 1.0) "/Game/JayCollab/Materials/M_Male_BodyYellow1.M_Male_BodyYellow1"))))))

(fn `F_SpawnAllPlayers`
  ;[1 1 1] GetMaxPlayers and loop through and add players according to max
  (`KismetSystemLibrary.PrintString` (`KismetStringLibrary.Conv_IntToString` (`self.MaxPlayerNumber`)))
  (for _index (range (`self.MaxPlayerNumber`))
    (set `self.PlayerIndex` _index)
    (for _array_element (`self.AllPlayerStarts`)
      (if (== (`PlayerStart.PlayerStartTag` _array_element) (`KismetStringLibrary.Conv_StringToName` (`KismetStringLibrary.Conv_IntToString` (`self.PlayerIndex`))))
        (`GameplayStatics.CreatePlayer` (`self.PlayerIndex`))
        (bind _returnvalue (`|SpawnActorFromClass` "/Game/JayCollab/BP_BaseCharacter.BP_BaseCharacter_C" (`self.GetTransform` _array_element) "Undefined" "OverrideRootScale" null null))
        (`Controller.Possess` (`GameplayStatics.GetPlayerController` (`self.PlayerIndex`)) _returnvalue)
        (`KismetArrayLibrary.Array_AddUnique` (`self.AllPlayers`) _returnvalue)
        ;;[1 0.7835 0] W.I.P
        (`self.F_SetPlayerColour` _returnvalue)
        (switch `int` (`self.PlayerIndex`)
          (:`0`
            (set `self.Player1Ref` _returnvalue))
          (:`1`
            (set `self.Player2Ref` _returnvalue))
          (:`2`
            (set `self.Player3Ref` _returnvalue))
          (:`3`
            (set `self.Player4Ref` _returnvalue)))))
    (bind _outactors (`GameplayStatics.GetAllActorsOfClass` "/Game/JayCollab/BP_BaseController.BP_BaseController_C"))
    (for _array_element_2 _outactors
      (`KismetArrayLibrary.Array_AddUnique` (`self.AllControllers`) _array_element_2))))

(fn `UserConstructionScript`)