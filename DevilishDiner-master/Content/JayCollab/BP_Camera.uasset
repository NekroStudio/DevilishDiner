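; BP_Camera is a shared camera for up to four players in Devilish Diner that keeps the group framed.
; After a brief BeginPlay delay, it caches players from GM_DevilishDiner and makes itself the view target for BP_BaseController actors.
; A fast looping timer, rather than Tick, sets spring arm length to the clamped largest pairwise player distance.
; The same update interpolates the camera actor toward the players' average location.
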(event `self.ReceiveBeginPlay`
  (`KismetSystemLibrary.Delay` 0.01)
  (`self.F_InitSetup`)
  (bind _returnvalue (`KismetSystemLibrary.K2_SetTimer` null "UpdateCamera" 0.001 true))
  (set `self.TimerHandle` _returnvalue))

(event `UpdateCamera`
  (`self.F_SetArmLengthForPlayers`)
  (`self.F_SetCameraPosForPlayers`))

(fn `F_GetPlayerLocations`
  (params (Player :type "/Game/JayCollab/BP_BaseCharacter Object Reference"))
  (returns (PlayerLoc :type "Vector Structure"))
  (locals (PlayerLocation :type "Vector Structure"))
  (`/Engine/EditorBlueprintResources/StandardMacros.IsValid` Player
    (:`Is Valid`
      (set `local.PlayerLocation` (`self.K2_GetActorLocation` Player)))
    (:`Is Not Valid`
      (set `local.PlayerLocation` (0.0 0.0 0.0))))
  (return (`local.PlayerLocation`)))

(fn `F_InitSetup`
  ;[1 1 1] Get all players
  (bind _asgm_devilish_diner (cast `/Game/JayCollab/GM_DevilishDiner` (`GameplayStatics.GetGameMode`)))
  (set `self.All PlayersRef` (`/Game/JayCollab/GM_DevilishDiner.AllPlayers` _asgm_devilish_diner))
  (bind _outactors (`GameplayStatics.GetAllActorsOfClass` "/Game/JayCollab/BP_BaseController.BP_BaseController_C"))
  (`PlayerController.SetViewTargetWithBlend` _outactors self 0.0 "VTBlend_Linear" 0.0 false)
  ;[1 1 1] Set all players in game to variables
  (for (_array_element _array_index) (`self.All PlayersRef`)
    (switch `int` _array_index
      (:`0`
        (set `self.Player1` _array_element))
      (:`1`
        (set `self.Player2` _array_element))
      (:`2`
        (set `self.Player3` _array_element))
      (:`3`
        (set `self.Player4` _array_element)))))

(fn `F_SetArmLengthDistance`
  (params (FirstPlayer :type "/Game/JayCollab/BP_BaseCharacter Object Reference") (SecondPlayer :type "/Game/JayCollab/BP_BaseCharacter Object Reference"))
  (returns (Distance :type "Float (double-precision)"))
  (locals (PlayerDistance :type "Float (double-precision)"))
  (if (and (`KismetSystemLibrary.IsValid` FirstPlayer) (`KismetSystemLibrary.IsValid` SecondPlayer))
    (set `local.PlayerDistance` (`self.GetDistanceTo` FirstPlayer SecondPlayer))
    (else
      (set `local.PlayerDistance` 0.0)))
  (return (`local.PlayerDistance`)))

(fn `F_SetArmLengthForPlayers`
  (bind _player1 (`self.Player1`))
  (bind _player2 (`self.Player2`))
  (bind _player3 (`self.Player3`))
  (bind _player4 (`self.Player4`))
  ;[1 1 1] Get the different distances between all players, clamp the arm length movement
  (set `SpringArmComponent.TargetArmLength` (`KismetMathLibrary.FClamp` (`.MaxValue` (`KismetMathLibrary.MaxOfFloatArray` (`|MakeArray` (`self.F_SetArmLengthDistance` _player1 _player2) (`self.F_SetArmLengthDistance` _player2 _player3) (`self.F_SetArmLengthDistance` _player2 _player4) (`self.F_SetArmLengthDistance` _player3 _player4) (`self.F_SetArmLengthDistance` _player1 _player3) (`self.F_SetArmLengthDistance` _player1 _player4)))) (`self.MinArmLength`) (`self.MaxArmLength`)) (`self.SpringArm`)))

(fn `F_SetCameraPosForPlayers`
  ;[1 1 1] Slightly adjust camera position to better suit all players on screen, slight interp for smoother movement
  (set `self.TargetPos` (/ (+ (`self.F_GetPlayerLocations` (`self.Player1`)) (`self.F_GetPlayerLocations` (`self.Player2`)) (`self.F_GetPlayerLocations` (`self.Player3`)) (`self.F_GetPlayerLocations` (`self.Player4`))) (`KismetMathLibrary.Conv_IntToDouble` (`KismetArrayLibrary.Array_Length` (`self.All PlayersRef`)))))
  (`self.K2_SetActorLocation` (`KismetMathLibrary.VInterpTo` (`self.CurrentPos`) (`self.TargetPos`) (`GameplayStatics.GetWorldDeltaSeconds`) (`self.InterpSpeed`)))
  (set `self.CurrentPos` (`self.K2_GetActorLocation`)))

(fn `UserConstructionScript`)