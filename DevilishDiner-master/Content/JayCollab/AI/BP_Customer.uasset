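; Customer AI character that gets a random guest mesh and a brief spawn effect on entering the level.
; Until the blackboard reports it is at a chair, a randomly re-timed timer drops random hazards with random yaw at its spawn point.
; Interface messages set and report happiness for particle FX, return the customer, and trigger exit by having the controller change behaviour tree and tagging it as leaving.
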(event `BeginSpawnLoop`
  ;[1 1 1] Loop random spawning of hazards when not sitting at table/chair
  (bind _returnvalue (`KismetSystemLibrary.K2_SetTimerDelegate` (delegate `SpawnHazard`) (`KismetMathLibrary.RandomFloatInRange` (`self.MinHazardSpawnLoop`) (`self.MaxHazardSpawnLoop`)) true :!label _label))
  (set `self.HazardSpawnHandle` _returnvalue))

(event `self.ReceiveBeginPlay`
  ;[1 1 1] Loop random spawning of hazards when not sitting at table/chair
  (`SkinnedMeshComponent.SetSkinnedAssetAndUpdate` (`self.Mesh`) (`self.M_GetRandomCustomerMesh`) true)
  (`|ExecutionSequence`
    (:`then_0`
      (goto _label))
    (:`then_1`
      ;[1 1 1] Spawn FX when customer enters level
      (bind _returnvalue (`NiagaraFunctionLibrary.SpawnSystemAtLocation` "/Game/JayCollab/FX/NS_CustomerSpawnFX.NS_CustomerSpawnFX" (`self.K2_GetActorLocation`) (struct) (0.5 0.5 0.5)))
      (`KismetSystemLibrary.Delay` 0.2)
      (`ActorComponent.Deactivate` _returnvalue))))

(event `SpawnHazard`
  ;[1 1 1] Loop random spawning of hazards when not sitting at table/chair
  (if (`self.M_CheckIfAtChair`)
    (`KismetSystemLibrary.K2_ClearAndInvalidateTimerHandle` (`self.HazardSpawnHandle`))
    (else
      (`|SpawnActorFromClass` (`self.M_GetRandomHazard`) (`self.M_RandRotTweakZaxis`) "AlwaysSpawn" "OverrideRootScale" null (struct :`R` 1.0 :`G` 1.0 :`B` 1.0 :`A` 1.0) null)
      (`KismetSystemLibrary.K2_ClearAndInvalidateTimerHandle` (`self.HazardSpawnHandle`))
      (`KismetSystemLibrary.Delay` 0.01)
      (`self.BeginSpawnLoop`))))

(event `/Game/JayCollab/AI/BPI_CustomerInterface.I_MessageCustomerExit`
  ;[1 1 1] Change behaviour tree through controller
  (message `/Game/JayCollab/AI/BPI_CustomerInterface.I_ChangeBehaviourTree` (`self.GetController`))
  (`KismetArrayLibrary.Array_Add` (`self.Tags`) "LeavingCustomer"))

(event `/Game/JayCollab/AI/BPI_CustomerInterface.I_CustomerIsHappy`
  ;[1 1 1] Check customer happiness for particle FX
  (set `self.CustomerHappy` true))

(fn `I_CheckCustomerIsHappy`
  (returns (CustomerHappy :type Boolean))
  (return (`self.CustomerHappy`)))

(fn `I_GetCustomer`
  (returns (Customer :type "/Game/JayCollab/AI/BP_Customer Object Reference"))
  (return self))

(fn `UserConstructionScript`)